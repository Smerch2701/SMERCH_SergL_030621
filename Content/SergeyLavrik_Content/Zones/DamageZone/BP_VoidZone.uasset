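; BP_VoidZone is a damage zone that hurts every actor inside its DamageZone collider.
; Begin and end overlap events add actors to and remove them from ArrayTargetActors.
; Tick applies the Damage value to each listed actor every frame, without delta-time scaling.
; The construction script sets ZoneMaterial on the DamageZone1 and DamageZone2 components.
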(event `self.ReceiveTick`
  (params (DeltaSeconds :type "Float (single-precision)"))
  ;[0 0 0] Нанесение урона Actor'ам из массива на которых получена ссылка
  (`KismetSystemLibrary.PrintString` (`KismetStringLibrary.Concat_StrStr` "Target: [" (`KismetSystemLibrary.GetDisplayName` (`self.TargetActorRef`)) "]") false false)
  (for _array_element (`self.ArrayTargetActors`)
    (`GameplayStatics.ApplyDamage` _array_element (`self.Damage`))))

(event `self.DamageZone.OnComponentBeginOverlap`
  (params (OverlappedComponent :type "PrimitiveComponent Object Reference") (OtherActor :type "Actor Object Reference") (OtherComp :type "PrimitiveComponent Object Reference") (OtherBodyIndex :type Integer) (bFromSweep :type Boolean) (SweepResult :type "HitResult Structure (by ref)"))
  ;[0 0 0] События коллайдера. Получение ссылки на Actor
  (`KismetArrayLibrary.Array_Add` (`self.ArrayTargetActors`) OtherActor))

(event `self.DamageZone.OnComponentEndOverlap`
  (params (OverlappedComponent :type "PrimitiveComponent Object Reference") (OtherActor :type "Actor Object Reference") (OtherComp :type "PrimitiveComponent Object Reference") (OtherBodyIndex :type Integer))
  ;[0 0 0] События коллайдера. Получение ссылки на Actor
  (`KismetArrayLibrary.Array_RemoveItem` (`self.ArrayTargetActors`) OtherActor))

(fn `UserConstructionScript`
  (`PrimitiveComponent.SetMaterial` (`self.DamageZone_2`) 0 (`self.ZoneMaterial`))
  (`PrimitiveComponent.SetMaterial` (`self.DamageZone_1`) 0 (`self.ZoneMaterial`)))