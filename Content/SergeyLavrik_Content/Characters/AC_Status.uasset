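; AC_Status is a character status component that tracks health as CurrentHP, starting at MaxHP on BeginPlay.
; MakeDamageHealth subtracts a given value from CurrentHP and clamps the result between zero and MaxHP.
; Tick prints the current HP on screen every frame as a debug readout.
; A delayed, looping self-damage test is left in the graph, disconnected from any event, so it never runs.
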(event `self.ReceiveBeginPlay`
  ;[0 0 0] Установка значения HP при создании персонажа
  (set `self.CurrentHP` (`self.MaxHP`)))

(event `self.ReceiveTick`
  (params (DeltaSeconds :type "Float (single-precision)"))
  ;[0 0 0] Вывод на экран текущее состояние HP
  (`KismetSystemLibrary.PrintString` (`KismetStringLibrary.Concat_StrStr` "Current HP: " (`KismetStringLibrary.Conv_DoubleToString` (`self.CurrentHP`))) true false (struct :`R` 0.01758 :`G` 0.473958 :`B` 0.027336 :`A` 1.0) DeltaSeconds))

(fn `MakeDamage/Health`
  (params (Value :type "Float (double-precision)"))
  (set `self.CurrentHP` (`KismetMathLibrary.FClamp` (- (`self.CurrentHP`) Value) 0.0 (`self.MaxHP`))))