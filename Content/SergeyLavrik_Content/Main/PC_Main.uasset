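; Player controller that creates the main HUD widget and handles game over, character selection and respawning.
; Every tick it pushes the pawn's health and stamina from AC_Status and weapon or lamp interaction hints to the widget.
; It polls health to toggle between gameplay and game-over screens, switching cursor and input mode.
; RestartPlayer spawns the selected Shooter, Healer or Recharger character at the first PlayerStart found and possesses it.
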(event `self.ReceiveBeginPlay`
  (`|ExecutionSequence`
    (:`then_0`
      ;[0 0 0] Создание WB_Main Widget
      (bind _returnvalue (`|CreateWidget` "/Game/SergeyLavrik_Content/UIX/WB_MainWidget.WB_MainWidget_C"))
      ;[0 0 0] Создание ссылки на Widget
      (bind _output_get (set `self.MainUIX` _returnvalue))
      ;[0 0 0] Вывод Виджета на экран
      (`UserWidget.AddToViewport` _output_get 0))
    (:`then_1`
      ;[0 0 0] Получение ссылки на персонажа (Управляемый Pawn)
      (bind _asch_main (cast `/Game/SergeyLavrik_Content/Characters/Ch_Main` (`self.K2_GetPawn`)))
      (set `self.MyPawn` _asch_main))))

(event `self.ReceiveTick`
  (params (DeltaSeconds :type "Float (single-precision)"))
  (bind _ac_status (`/Game/SergeyLavrik_Content/Characters/Ch_Main.AC_Status` (`self.MyPawn`)))
  (bind _ac_status_2 (`/Game/SergeyLavrik_Content/Characters/Ch_Main.AC_Status` (`self.MyPawn`)))
  (bind _interactweapon (`/Game/SergeyLavrik_Content/Characters/Ch_Main.InteractWeapon` (`self.MyPawn`)))
  (`|ExecutionSequence`
    (:`then_0`
      ;[0 0 0] Получение значений HP из компонента персонажа AC_Status
      (`/Game/SergeyLavrik_Content/UIX/WB_MainWidget.UpdateHealth` (`self.MainUIX`) (`/Game/SergeyLavrik_Content/Characters/AC_Status.CurrentHP` _ac_status) (`/Game/SergeyLavrik_Content/Characters/AC_Status.MaxHP` _ac_status)))
    (:`then_1`
      ;[0 0 0] Получение значений Stamina из компонента персонажа AC_Status
      (`/Game/SergeyLavrik_Content/UIX/WB_MainWidget.UpdateStamina` (`self.MainUIX`) (`/Game/SergeyLavrik_Content/Characters/AC_Status.CurrentStamina` _ac_status_2) (`/Game/SergeyLavrik_Content/Characters/AC_Status.MaxStamina` _ac_status_2)))
    (:`then_2`
      ;[0 0 0] Подсказки для интерактивных объектов (Hint Interaction Objects)
      (if (`KismetSystemLibrary.IsValid` _interactweapon)
        (`/Game/SergeyLavrik_Content/UIX/WB_MainWidget.UpdateInteract` (`self.MainUIX`) (`KismetStringLibrary.Conv_NameToString` (`/Game/SergeyLavrik_Content/Weapons/Weapon_Gun/BP_WeaponBaseGun.WeaponName` _interactweapon)))
        (elif (`KismetSystemLibrary.IsValid` (`/Game/SergeyLavrik_Content/Characters/Ch_Main.InteractLamp` (`self.MyPawn`)))
          (`/Game/SergeyLavrik_Content/UIX/WB_MainWidget.UpdateInteract` (`self.MainUIX`) "Activate")
          (else
            (`/Game/SergeyLavrik_Content/UIX/WB_MainWidget.PlayHintAnimation` (`self.MainUIX`) true)
            (`/Game/SergeyLavrik_Content/UIX/WB_MainWidget.UpdateInteract` (`self.MainUIX`) "")))))
    (:`then_3`
      ;[0 0 0] Проверка текущего состояния здоровья игрока
      (if (`self.PlayerAlive`)
        (if (<= (`/Game/SergeyLavrik_Content/Characters/AC_Status.CurrentHP` (`/Game/SergeyLavrik_Content/Characters/Ch_Main.AC_Status` (`self.MyPawn`))) 0.0)
          (set `self.PlayerAlive` false)
          (`/Game/SergeyLavrik_Content/UIX/WB_MainWidget.SwitchScreen` (`self.MainUIX`) 1)
          (set `self.bShowMouseCursor` true)
          (`/Game/SergeyLavrik_Content/UIX/WB_MainWidget.PlayGameOverAnimation` (`self.MainUIX`))
          (`WidgetBlueprintLibrary.SetInputMode_UIOnlyEx` self (`self.MainUIX`)))
        (elif (> (`/Game/SergeyLavrik_Content/Characters/AC_Status.CurrentHP` (`/Game/SergeyLavrik_Content/Characters/Ch_Main.AC_Status` (`self.MyPawn`))) 0.0)
          (set `self.PlayerAlive` true)
          (`/Game/SergeyLavrik_Content/UIX/WB_MainWidget.SwitchScreen` (`self.MainUIX`) 0)
          (set `self.bShowMouseCursor` false)
          (`WidgetBlueprintLibrary.SetInputMode_GameOnly` self))))))

(event `OpenCharacterSelector`
  ;[0 0 0] Переключение на окно выбора персонажа
  ;;[0 0 0] Переключение на виджет с индексом 2(Character Selection Window)
  (`/Game/SergeyLavrik_Content/UIX/WB_MainWidget.SwitchScreen` (`self.MainUIX`) 2))

(event `RestartPlayer`
  ;[0 0 0] Перерождение персонажа
  (`KismetSystemLibrary.PrintString` "Spawn Player" true false (struct :`R` 1.0 :`G` 0.470479 :`A` 1.0))
  ;;[0 0 0] Выбор персонажа для возрождения
  (switch `/Game/SergeyLavrik_Content/Enums/E_CharacterSelector` (`self.SelectCharacter`)
    (:`NewEnumerator0`
      (set `self.CurrentCharacter` "/Game/SergeyLavrik_Content/Characters/Ch_Main.Ch_Main_C"))
    (:`NewEnumerator1`
      (set `self.CurrentCharacter` "/Game/SergeyLavrik_Content/Characters/Ch_HealerMan_Child.Ch_HealerMan_Child_C"))
    (:`NewEnumerator2`
      (set `self.CurrentCharacter` "/Game/SergeyLavrik_Content/Characters/Ch_Recharger_Child.Ch_Recharger_Child_C")))
  ;;[0 0 0] Вывод на экран уведомления о выбранном персонаже
  (`KismetSystemLibrary.PrintString` (`KismetStringLibrary.Concat_StrStr` "Selected character: " (`|GetEnumeratorNameAsString` (`self.SelectCharacter`))) true false (struct :`R` 0.026286 :`G` 0.296875 :`B` 0.05322 :`A` 1.0))
  ;;[0 0 0] Проверка всех Actor'ов класса PlayerStart, получение их расположения и создание Actor'а класса Ch_Main на месте полученного PlayerStart
  (bind _outactors (`GameplayStatics.GetAllActorsOfClass` "/Script/Engine.PlayerStart"))
  (bind _returnvalue (`|SpawnActorFromClass` (`self.CurrentCharacter`) (`self.GetTransform` (`|GetArrayItem` _outactors)) "AlwaysSpawn" "OverrideRootScale" null null))
  ;;[0 0 0] Запись созданного Ch_Main в переменную MyPawn
  (set `self.MyPawn` _returnvalue)
  ;;[0 0 0] Открепляем контроллер от старого персонажа
  (`self.UnPossess`)
  ;;[0 0 0] Прикрепляем контроллер к новому персонажу записанному в ссылке
  (`self.Possess` (`self.MyPawn`)))

(fn `UserConstructionScript`)