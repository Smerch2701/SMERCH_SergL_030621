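; Laser gun weapon that deals continuous damage to whatever its beam hits while active.
; Its override of the base Fire event toggles LaserActive, which Tick checks every frame.
; While active, an object-type line trace from the Arrow applies frame-time-scaled damage and moves the particle effect to the impact point.
; The effect deactivates without a hit; the beam only appears as a debug trace line, alongside debug state prints.
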(event `self.ReceiveTick`
  (params (DeltaSeconds :type "Float (single-precision)"))
  (bind _arrow (`self.Arrow`))
  (bind _returnvalue (`SceneComponent.K2_GetComponentLocation` _arrow))
  ;[0 0 0] Проверка активации лазера
  (if (`self.LaserActive`)
    (`KismetSystemLibrary.PrintString` "Laser Activated.." true false (struct :`R` 1.0 :`G` 0.51859 :`B` 0.072215 :`A` 1.0) 0.001)
    ;[0 0 0] Трассировка луча в пространстве по заданным координатам
    (bind (_outhit _returnvalue_2) (`KismetSystemLibrary.LineTraceSingleForObjects` :`Start` _returnvalue :`End` (+ _returnvalue (* (`SceneComponent.GetForwardVector` _arrow) 10000.0)) :`ObjectTypes` (`|MakeArray` "ObjectTypeQuery1" "ObjectTypeQuery4" "ObjectTypeQuery3" :!type "EObjectTypeQuery Enum") :`DrawDebugType` "ForOneFrame"))
    ;[0 0 0] Активация/Дизактивация системы частиц
    (if _returnvalue_2
      (`ActorComponent.Activate` (`self.ParticleSystem`) false)
      (bind (_bblockinghit _binitialoverlap _time _distance _location _impactpoint _normal _impactnormal _physmat _hitactor) (`GameplayStatics.BreakHitResult` _outhit))
      ;[0 0 0] Перемещение Particle System к точке столкновения
      (`SceneComponent.K2_SetWorldLocation` (`self.ParticleSystem`) _impactpoint false false)
      ;[0 0 0] Нанесение урона
      (`GameplayStatics.ApplyDamage` _hitactor (* (`self.Damage`) (`GameplayStatics.GetWorldDeltaSeconds`)) null self)
      (else
        (`ActorComponent.Deactivate` (`self.ParticleSystem`))))
    (else
      ;[0 0 0] Дизактивация эффекта частиц
      (`ActorComponent.Deactivate` (`self.ParticleSystem`))
      (`KismetSystemLibrary.PrintString` "Laser Disactivated.." true false (struct :`R` 0.140625 :`G` 0.140625 :`B` 0.140625 :`A` 1.0) 0.001))))

(event `self.Fire`
  (params (ActivateGun :type Boolean))
  ;[0 0 0] Перегрузка базовой функции
  (set `self.LaserActive` ActivateGun))

(fn `UserConstructionScript`
  (`parent.UserConstructionScript`))