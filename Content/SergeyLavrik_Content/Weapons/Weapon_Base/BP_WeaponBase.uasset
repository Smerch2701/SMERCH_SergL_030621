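; BP_WeaponBase is a base weapon actor that automatically attempts to fire once per second from BeginPlay.
; When CanFire is set, Fire checks and subtracts one round through the ACAmmo component, then spawns BP_AmmoBase and a briefly activated steam emitter at the Arrow component.
; With insufficient ammo it plays a click sound instead.
; Either way, a text render then shows current and maximum ammo.
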(event `self.ReceiveBeginPlay`
  (`KismetSystemLibrary.Delay` 1.0 :!label _label)
  (`self.Fire`)
  (goto _label))

(event `Fire`
  (bind _ac_ammo (`self.AC_Ammo`))
  (bind _ac_ammo_2 (`self.AC_Ammo`))
  (if (`self.CanFire`)
    (`|ExecutionSequence`
      (:`then_0`
        ;[0 0 0] Выполнение функции подсчёта боеприпасов при вызове события Fire
        (if (`/Game/SergeyLavrik_Content/Weapons/Weapon_Base/AC_Ammo.F_CheckAmmo` _ac_ammo 1)
          (`/Game/SergeyLavrik_Content/Weapons/Weapon_Base/AC_Ammo.F_SubtractAmmo` _ac_ammo 1)
          ;[0 0 0] Создание экземпляра класса BP_AmmoBase
          (`|SpawnActorFromClass` "/Game/SergeyLavrik_Content/Weapons/Weapon_Base/BP_AmmoBase.BP_AmmoBase_C" (`SceneComponent.K2_GetComponentToWorld` (`self.Arrow`)) "AlwaysSpawn" "OverrideRootScale" null null)
          ;[0 0 0] Создание эмиттера частиц в области выстрела
          (bind _returnvalue (`GameplayStatics.SpawnEmitterAtLocation` "/Game/DownloadContent/StarterContent/Particles/P_Steam_Lit.P_Steam_Lit" (`SceneComponent.K2_GetComponentLocation` (`self.Arrow`)) (struct) (0.2 0.2 0.2)))
          (`ActorComponent.Deactivate` _returnvalue)
          (else
            ;;[0 0 0] Создание звука при нехватке боезапаса
            (`GameplayStatics.SpawnSoundAtLocation` "/Engine/VREditor/Sounds/UI/Click_on_Button_Cue.Click_on_Button_Cue" (`self.K2_GetActorLocation`) (struct) 1.0 1.0 0.0 null null))))
      (:`then_1`
        ;[0 0 0] Вывод значений боезапаса в TextRender_Ammo
        (`TextRenderComponent.K2_SetText` (`self.TextRender_Ammo`) (`|FormatText` "{Current}/{Max}" (`/Game/SergeyLavrik_Content/Weapons/Weapon_Base/AC_Ammo.CurrentAmmo` _ac_ammo_2) (`/Game/SergeyLavrik_Content/Weapons/Weapon_Base/AC_Ammo.MaxAmmo` _ac_ammo_2)))))))

(fn `UserConstructionScript`)