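; Actor component that tracks a weapon's ammo count for the weapon base.
; It fills current ammo to the maximum on BeginPlay.
; A subtract function lowers the count by a given amount, clamped between zero and the maximum, and a check function reports whether enough ammo remains for a requested amount.
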(event `self.ReceiveBeginPlay`
  ;[0 0 0] Установка полного боезопаса в начале игры
  (set `self.CurrentAmmo` (`self.MaxAmmo`)))

(fn `F_CheckAmmo`
  (params (Value :type Integer :default 1))
  (returns (ReturnValue :type Boolean))
  ;[0 0 0] Проверка количества боезапаса
  (return (>= (`self.CurrentAmmo`) Value)))

(fn `F_SubtractAmmo`
  (params (Value :type Integer :default 1))
  ;[0 0 0] Отнять от Current Ammo значение Value при вызове функции
  (set `self.CurrentAmmo` (`KismetMathLibrary.Clamp` (- (`self.CurrentAmmo`) Value) 0 (`self.MaxAmmo`))))