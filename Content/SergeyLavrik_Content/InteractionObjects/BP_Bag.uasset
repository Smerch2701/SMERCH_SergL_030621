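; BP_Bag is an interaction object that briefly flashes red when something hits it.
; A component hit on one of its cylinders turns Cylinder4 red, then Cylinder2, then restores each to the bag material in the same order, staggered by short delays.
; The hit actor's name feeds a Print String with screen and log output both switched off.
; Construction script, BeginPlay, overlap and Tick do nothing.
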(event `self.Cylinder_4.OnComponentHit`
  (params (HitComponent :type "PrimitiveComponent Object Reference") (OtherActor :type "Actor Object Reference") (OtherComp :type "PrimitiveComponent Object Reference") (NormalImpulse :type "Vector Structure") (Hit :type "HitResult Structure (by ref)"))
  (`KismetSystemLibrary.PrintString` (`KismetStringLibrary.Concat_StrStr` "Actor Hit: [" (`KismetSystemLibrary.GetDisplayName` OtherActor) "]") false false (struct :`G` 0.66 :`B` 1.0 :`A` 1.0) 0.2)
  ;[0 0 0] Изменение цвета элементов при столкновении с Actor'ом
  (`PrimitiveComponent.SetMaterial` (`self.Cylinder_4`) 0 "/Game/SergeyLavrik_Content/Materials/Red_ButtonMaterial_Inst.Red_ButtonMaterial_Inst")
  (`KismetSystemLibrary.Delay` 0.2)
  (`PrimitiveComponent.SetMaterial` (`self.Cylinder_2`) 0 "/Game/SergeyLavrik_Content/Materials/Red_ButtonMaterial_Inst.Red_ButtonMaterial_Inst")
  (`KismetSystemLibrary.Delay` 0.2)
  (`PrimitiveComponent.SetMaterial` (`self.Cylinder_4`) 0 "/Game/SergeyLavrik_Content/Materials/Bag_Material1.Bag_Material1")
  (`KismetSystemLibrary.Delay` 0.2)
  (`PrimitiveComponent.SetMaterial` (`self.Cylinder_2`) 0 "/Game/SergeyLavrik_Content/Materials/Bag_Material1.Bag_Material1"))

(fn `UserConstructionScript`)