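; Base elevator interaction object that moves a platform along a spline when activated and back when deactivated.
; The overridden ActivateInteract calls its parent, then plays or reverses the MovingScale timeline based on OnActive.
; Each timeline update samples the spline by time to set the platform's world location and yaw-only rotation, keeping it level, and prints the current value on screen for debugging.
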(event `self.ActivateInteract`
  (params (OnActive :type Boolean))
  ;[0 0 0] Перегрузка родительской функции
  (`parent.ActivateInteract` OnActive)
  ;[0 0 0] Проверка активации лифта
  (if (`self.OnActive`)
    ;[0 0 0] TimeLine движения лифта
    (bind (_direction _movingscale) (`Timeline|MovingScale` :!label _label)
      (:`Update`
        (`KismetSystemLibrary.PrintString` (`KismetStringLibrary.Concat_StrStr` "Elevator.MovingScale: [" (`KismetStringLibrary.Conv_DoubleToString` _movingscale) "]") true false (struct :`G` 0.66 :`B` 1.0 :`A` 1.0) 0.01)
        ;[0 0 0] Обновление координат платформы в мировых координатах
        ;;[0 0 0] Перемещение ElevatorPlatform по Spline
        (`SceneComponent.K2_SetWorldLocation` (`self.ElevatorPlatform`) (`SplineComponent.GetLocationAtTime` (`self.Spline`) _movingscale "World" false) false false)
        ;;[0 0 0] Поворот ElevatorPlatform по Spline
        (`SceneComponent.K2_SetWorldRotation` (`self.ElevatorPlatform`) (`KismetMathLibrary.MakeRotator` 0.0 0.0 (.yaw (`SplineComponent.GetRotationAtTime` (`self.Spline`) _movingscale "World" false))) false false)))
    (else
      (goto _label :!via `Reverse`))))

(fn `UserConstructionScript`
  (`parent.UserConstructionScript`))