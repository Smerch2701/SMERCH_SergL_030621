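; BP_WeaponHolder is an interactive weapon rack with one working slot that takes the player's active weapon.
; Overlapping its box stores Ch_Main's ActiveWeapon, then, if the slot is empty and CanAttach is set, snaps it to WeaponMaket1 and marks it Reserved.
; DetachWeapon clears the slot and reference.
; Tick prints debug state, recolors the middle indicator by occupancy and flickers the outer two as faulty using random Delays.
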(event `self.ReceiveTick`
  (params (DeltaSeconds :type "Float (single-precision)"))
  ;[0 0 0] Текущее оружие записанное в ячейку WeaponHolder
  (`KismetSystemLibrary.PrintString` (`KismetStringLibrary.Concat_StrStr` "Place1 Attached Weapon: [" (`KismetSystemLibrary.GetDisplayName` (`self.AttachedWeapon_Ref`)) "]") true false (struct :`R` 0.056128 :`G` 0.309469 :`B` 1.0 :`A` 1.0) DeltaSeconds)
  ;[0 0 0] Состояние ячейки под оружие Занято или Пусто
  (`KismetSystemLibrary.PrintString` (`KismetStringLibrary.Concat_StrStr` "Place1: [" (`|GetEnumeratorNameAsString` (`self.Place1`)) "]") true false (struct :`R` 0.039546 :`G` 0.55834 :`B` 0.174647 :`A` 1.0) DeltaSeconds)
  ;[0 0 0] Смена цвета индикатора на держателе при закреплении/подборе оружия
  (`|ExecutionSequence`
    (:`then_0`
      (if (`|EnumEquality` (`self.Place1`) "NewEnumerator1")
        (`PrimitiveComponent.SetMaterial` (`self.HolderIndicator2`) 0 "/Game/SergeyLavrik_Content/Materials/Green_ButtonMaterial_Inst.Green_ButtonMaterial_Inst")))
    (:`then_1`
      (if (`|EnumEquality` (`self.Place1`) "NewEnumerator0")
        (`PrimitiveComponent.SetMaterial` (`self.HolderIndicator2`) 0 "/Game/SergeyLavrik_Content/Materials/ButtonMaterial.ButtonMaterial")))
    (:`then_2`
      ;[0 0 0] Эффект мигания неисправных индикаторов ячеек BP_WeaponHolder
      (`KismetSystemLibrary.Delay` (`KismetMathLibrary.RandomFloatInRange` 0.0 0.5))
      (`PrimitiveComponent.SetMaterial` (`self.HolderIndicator1`) 0 "/Game/SergeyLavrik_Content/Materials/ButtonMaterial.ButtonMaterial")
      (`PrimitiveComponent.SetMaterial` (`self.HolderIndicator3`) 0 "/Game/SergeyLavrik_Content/Materials/ButtonMaterial.ButtonMaterial")
      (`KismetSystemLibrary.Delay` (`KismetMathLibrary.RandomFloatInRange` 0.0 0.5))
      (`PrimitiveComponent.SetMaterial` (`self.HolderIndicator1`) 0 "/Game/SergeyLavrik_Content/Materials/Inactive_ButtonMaterial_Inst.Inactive_ButtonMaterial_Inst")
      (`PrimitiveComponent.SetMaterial` (`self.HolderIndicator3`) 0 "/Game/SergeyLavrik_Content/Materials/Inactive_ButtonMaterial_Inst.Inactive_ButtonMaterial_Inst"))))

(event `self.BoxCollision1.OnComponentBeginOverlap`
  (params (OverlappedComponent :type "PrimitiveComponent Object Reference") (OtherActor :type "Actor Object Reference") (OtherComp :type "PrimitiveComponent Object Reference") (OtherBodyIndex :type Integer) (bFromSweep :type Boolean) (SweepResult :type "HitResult Structure (by ref)"))
  ;[0 0 0] Запись текущей ссылки на оружие в руках персонажа в ссылку WeaponHolder
  (bind _asch_main (cast `/Game/SergeyLavrik_Content/Characters/Ch_Main` OtherActor))
  (set `self.AttachedWeapon_Ref` (`/Game/SergeyLavrik_Content/Characters/Ch_Main.ActiveWeapon` _asch_main))
  ;[0 0 0] Проверка состояния ячейки Пустая или Занята
  (switch `/Game/SergeyLavrik_Content/Enums/E_WeaponHolderCheckPlace` (`self.Place1`)
    (:`NewEnumerator0`
      (if (`self.CanAttach`)
        (`self.AttachWeapon`)))))

(event `AttachWeapon`
  ;[0 0 0] Прикрепить оружие к держателю для оружий(WeaponHolder) если оружие находится в руках у игрока
  (`self.F_AttachWeapon`))

(event `DetachWeapon`
  ;[0 0 0] При откреплении оружия от держателя сменить состояние ячейки Занято на Пусто
  (set `self.Place1` "NewEnumerator0")
  (set `self.AttachedWeapon_Ref` null))

(fn `F_AttachWeapon`
  (if (`KismetSystemLibrary.IsValid` (`self.AttachedWeapon_Ref`))
    (if (`|EnumEquality` (`self.Place1`) "NewEnumerator0")
      (`self.SetActorEnableCollision` (`self.AttachedWeapon_Ref`) true)
      ;[0 0 0] Прикрепить ActiveWeapon к компоненту WeaponMaket1
      (`self.K2_AttachToComponent` (`self.AttachedWeapon_Ref`) (`self.WeaponMaket1`) "None" "SnapToTarget" "SnapToTarget" "SnapToTarget" true)
      (set `self.Place1` "NewEnumerator1"))))

(fn `UserConstructionScript`)