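; Elevator actor that moves its platform vertically between levels selected by an enum state.
; Tick switches on that state, stepping a tracked height by a fixed per-frame speed, unscaled by delta time, and applying it through a relative-offset function.
; A numeric Level gates moves to levels 1 and 2 and scales the level 3 limit.
; Reaching a limit sets the state inactive; DoOnce nodes print debug status.
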(event `self.ReceiveTick`
  (params (DeltaSeconds :type "Float (single-precision)"))
  (switch `/Game/SergeyLavrik_Content/Enums/E_ElevatorLevel` (`self.ElevatorLevel`)
    (:`NewEnumerator0`
      ;[0 0 0] Возвращаем Elevator на первый уровень
      (if (== (`self.Level`) 2.0)
        ;[0 0 0] Elevator Level 1
        (if (> (`self.ElevatorLocation`) 0.0)
          (bind _output_get (set `self.ElevatorLocation` (- (`self.ElevatorLocation`) (`self.ElevatorSpeed`))))
          (`self.F_ElevatorLocation` (* (`self.ElevatorSpeed`) -1.0))
          (`/Engine/EditorBlueprintResources/StandardMacros.DoOnce` false
            (:`Completed`
              (`KismetSystemLibrary.PrintString` (`KismetStringLibrary.Concat_StrStr` "Elevator Location: " (`KismetStringLibrary.Conv_DoubleToString` _output_get) "; Elevator Level: " (`|GetEnumeratorNameAsString` (`self.ElevatorLevel`))) true false (struct :`R` 1.0 :`G` 0.47074 :`B` 0.026278 :`A` 1.0))))
          (else
            (set `self.ElevatorLevel` "NewEnumerator2")))
        (else
          (set `self.Level` 2.0))))
    (:`NewEnumerator1`
      (if (== (`self.Level`) 1.0)
        ;[0 0 0] Elevator Level 2
        (if (< (`self.ElevatorLocation`) (`self.ElevatorMaxLocation`))
          (bind _output_get_2 (set `self.ElevatorLocation` (+ (`self.ElevatorLocation`) (`self.ElevatorSpeed`))))
          (`self.F_ElevatorLocation` (`self.ElevatorSpeed`))
          (`/Engine/EditorBlueprintResources/StandardMacros.DoOnce` false
            (:`Completed`
              (`KismetSystemLibrary.PrintString` (`KismetStringLibrary.Concat_StrStr` "Elevator Location: " "" "; Elevator Level: " (`|GetEnumeratorNameAsString` (`self.ElevatorLevel`))) true false (struct :`R` 1.0 :`G` 0.47074 :`B` 0.026278 :`A` 1.0))))
          (else
            (set `self.ElevatorLevel` "NewEnumerator2")))
        (else
          (set `self.ElevatorLevel` "NewEnumerator0"))))
    (:`NewEnumerator3`
      ;[0 0 0] Elevator Level 3
      (if (< (`self.ElevatorLocation`) (* (`self.ElevatorMaxLocation`) (`self.Level`)))
        (bind _output_get_3 (set `self.ElevatorLocation` (+ (`self.ElevatorLocation`) (`self.ElevatorSpeed`))))
        (`self.F_ElevatorLocation` (`self.ElevatorSpeed`))
        (`/Engine/EditorBlueprintResources/StandardMacros.DoOnce` false
          (:`Completed`
            (`KismetSystemLibrary.PrintString` (`KismetStringLibrary.Concat_StrStr` "Elevator Location: " "" "; Elevator Level: " (`|GetEnumeratorNameAsString` (`self.ElevatorLevel`))) true false (struct :`R` 1.0 :`G` 0.473531 :`B` 0.026241 :`A` 1.0))))
        (else
          (set `self.ElevatorLevel` "NewEnumerator2"))))))

(fn `F_ElevatorLocation`
  (params (`Elevator Speed` :type "Float (double-precision)"))
  (`SceneComponent.K2_AddRelativeLocation` (`self.ElevatorPlatform`) (`KismetMathLibrary.MakeVector` 0.0 0.0 `Elevator Speed`) false false))

(fn `UserConstructionScript`)