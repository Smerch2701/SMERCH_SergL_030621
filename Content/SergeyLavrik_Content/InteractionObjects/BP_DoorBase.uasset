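; BP_DoorBase is an interactable door that swings open on activation and closes itself after a delay.
; ActivateInteract extends the parent's logic, then passes its active flag to OpenDoor, which stores the open/closed state.
; OpenDoor plays or reverses the DoorAngle timeline, whose updates set the Door component's relative yaw.
; When the timeline finishes with the door still open, a five-second delay precedes the automatic close.
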(event `self.ReceiveBeginPlay`)

(event `self.ReceiveTick`
  (params (DeltaSeconds :type "Float (single-precision)")))

(event `OpenDoor`
  (params (Open :type Boolean))
  ;[0 0 0] Создание события открытия двери по Time Line
  ;;[0 0 0] Состояние двери Открыто/Закрыто
  (bind _output_get (set `self.Open/Close` Open))
  (if _output_get
    (bind (_direction _angle) (`Timeline|DoorAngle` :!label _label)
      (:`Update`
        (`KismetSystemLibrary.PrintString` (`KismetStringLibrary.Concat_StrStr` "DoorAngle: " (`KismetStringLibrary.Conv_DoubleToString` _angle)) false false)
        ;[0 0 0] Указание на вращение компонента Door относительно указанной оси
        (`SceneComponent.K2_SetRelativeRotation` (`self.Door`) (`KismetMathLibrary.MakeRotator` 0.0 0.0 _angle) false false))
      (:`Finished`
        ;[0 0 0] Запуск TimeLine в обратном режиме (Revers)
        (if (`self.Open/Close`)
          ;;[0 0 0] Закрыть дверь если она осталась открыта
          (`KismetSystemLibrary.Delay` 5.0)
          (`self.OpenDoor` false))))
    (else
      (goto _label :!via `Reverse`))))

(event `self.ActivateInteract`
  (params (OnActive :type Boolean))
  ;[0 0 0] Перегрузка родительской функции
  ;[0 0 0] Вызов логики родительского объекта
  (`parent.ActivateInteract` OnActive)
  ;[0 0 0] Вызов события открытия двери
  (`self.OpenDoor` OnActive))

(fn `UserConstructionScript`)