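; Interactable lamp Blueprint whose light turns on or off when it is activated.
; It overrides the ActivateInteract event, printing an on-screen debug message and passing the active flag to F_SwitchLight.
; F_SwitchLight toggles the PointLight by setting its intensity to a fixed bright value or to zero.
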(event `self.ReceiveBeginPlay`)

(event `self.ReceiveTick`
  (params (DeltaSeconds :type "Float (single-precision)")))

(event `self.ActivateInteract`
  (params (OnActive :type Boolean))
  ;[0 0 0] Перегруженное событие активации
  (`KismetSystemLibrary.PrintString` "Activated object" true false (struct :`R` 0.012997 :`G` 0.259747 :`B` 1.0 :`A` 1.0))
  (`self.F_SwitchLight` OnActive))

(fn `F_SwitchLight`
  (params (`On/Off` :type Boolean))
  ;[0 0 0] Функция Включения/Выключения лампы
  (set `self.On/Off` `On/Off`)
  (if (`self.On/Off`)
    (`LightComponent.SetIntensity` (`self.PointLight`) 15000.0)
    (return)
    (else
      (`LightComponent.SetIntensity` (`self.PointLight`) 0.0)
      (return))))

(fn `UserConstructionScript`)