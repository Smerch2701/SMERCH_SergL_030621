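; BP_HoverPlatform is a physics-driven platform that hovers above static world geometry.
; Each Tick it line-traces 600 units down from the Platform component against WorldStatic objects.
; On a hit it applies an upward, mass-independent force that grows as the surface gets closer, acting like an undamped-by-script spring.
; The trace and on-screen prints of proximity and hit state serve as debug output.
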(event `self.ReceiveTick`
  (params (DeltaSeconds :type "Float (single-precision)"))
  ;[0 0 0] Отрисовка проецируемого луча в пространстве
  (bind (_outhit _returnvalue) (`KismetSystemLibrary.LineTraceSingleForObjects` :`Start` (`SceneComponent.K2_GetComponentLocation` (`self.Platform`)) :`End` (+ (`SceneComponent.K2_GetComponentLocation` (`self.Platform`)) (0.0 0.0 -600.0)) :`ObjectTypes` (`|MakeArray` "ObjectTypeQuery1" :!type "EObjectTypeQuery Enum") :`DrawDebugType` "ForOneFrame"))
  (bind _returnvalue_2 (- 1.0 (`.Time` (`GameplayStatics.BreakHitResult` _outhit))))
  (`KismetSystemLibrary.PrintString` (`KismetStringLibrary.Concat_StrStr` "% Distance platform: " (`KismetStringLibrary.Conv_DoubleToString` _returnvalue_2)) true false)
  ;[0 0 0] Проверка на наличие других объектов пересекающих Line Trace
  (`KismetSystemLibrary.PrintString` (`KismetStringLibrary.Concat_StrStr` "Other Actors " (`KismetStringLibrary.Conv_BoolToString` _returnvalue)) true false (struct :`G` 0.66 :`B` 1.0 :`A` 1.0) DeltaSeconds)
  (if _returnvalue
    ;[0 0 0] Применение силы в указанном направлении компоненту
    (`PrimitiveComponent.AddForce` (`self.Platform`) (* (0.0 0.0 1500.0) _returnvalue_2) "None" true)))

(fn `UserConstructionScript`)