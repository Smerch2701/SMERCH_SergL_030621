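; Base lamp Blueprint whose point light flickers between warm yellow, blue and off.
; Tick fires two custom events that drive the same PointLight, each throttled by a Delay and alternating on and off through a FlipFlop.
; LightEvent1 gives a steady-interval yellow blink, while LightEvent2 adds blue flashes at random intervals and brightness.
; FSwitchLight sets the intensity; FTestFunction is an empty stub.
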(event `self.ReceiveBeginPlay`)

(event `self.ReceiveTick`
  (params (DeltaSeconds :type "Float (single-precision)"))
  (`self.LightEvent1`)
  (`self.LightEvent2`))

(event `LightEvent1`
  ;[0 0 0] LightEvents
  (`KismetSystemLibrary.Delay` 2.0)
  (`/Engine/EditorBlueprintResources/StandardMacros.FlipFlop`
    (:`A`
      (`self.F_SwitchLight` 20000.0)
      (`LightComponent.SetLightColor` (`self.PointLight`) (struct :`R` 1.0 :`G` 1.0 :`B` 0.473531 :`A` 1.0) true)
      (`KismetSystemLibrary.Delay` 4.0))
    (:`B`
      (`self.F_SwitchLight` 0.0))))

(event `LightEvent2`
  ;[0 0 0] LightEvents
  (`KismetSystemLibrary.Delay` (`KismetMathLibrary.RandomFloatInRange` 0.1 2.0))
  (`/Engine/EditorBlueprintResources/StandardMacros.FlipFlop`
    (:`A`
      (`self.F_SwitchLight` (`KismetMathLibrary.RandomFloatInRange` 0.0 20000.0))
      (`LightComponent.SetLightColor` (`self.PointLight`) (struct :`R` 0.131722 :`G` 0.135433 :`B` 1.0 :`A` 1.0) true))
    (:`B`
      (`self.F_SwitchLight` 0.0))))

(fn `F Test Function`)

(fn `F_SwitchLight`
  (params (Intensity :type "Float (double-precision)"))
  (`LightComponent.SetIntensity` (`self.PointLight`) Intensity)
  (return))

(fn `UserConstructionScript`)