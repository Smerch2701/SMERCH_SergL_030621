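; BP_ElevatorFloor is an elevator floor piece that slides along its relative X axis for level 2 or 3, with welcome text set at BeginPlay.
; Tick switches on SwitchOpenLevel, checks the matching floor level and location limit, then steps the floor by negative speed through FElevatorFloorLocation.
; The tracked location decreases for level 2 but increases for level 3, although both move the component in the same direction.
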(event `self.ReceiveBeginPlay`
  (`TextRenderComponent.K2_SetText` (`self.TextRender`) (`self.WelcomeText`)))

(event `self.ReceiveTick`
  (params (DeltaSeconds :type "Float (single-precision)"))
  (switch `/Game/SergeyLavrik_Content/Enums/E_ElevatorLevel` (`self.SwitchOpenLevel`)
    (:`NewEnumerator1`
      ;[0 0 0] Open Level 2
      (if (== (`self.ElevatorFloorLevel`) 2.0)
        (if (> (`self.ElevatorFloorLocation`) (`self.ElevatorFloorMaxLocation`))
          (set `self.ElevatorFloorLocation` (+ (`self.ElevatorFloorLocation`) (* (`self.SpeedElevatorFloor`) -1.0)))
          (`self.F_ElevatorFloor_Location` (* (`self.SpeedElevatorFloor`) -1.0)))))
    (:`NewEnumerator3`
      ;[0 0 0] Open Level 3
      (if (== (`self.ElevatorFloorLevel`) 3.0)
        (if (> (`self.ElevatorFloorLocation`) (`self.ElevatorFloorMaxLocation`))
          (set `self.ElevatorFloorLocation` (+ (`self.ElevatorFloorLocation`) (`self.SpeedElevatorFloor`)))
          (`self.F_ElevatorFloor_Location` (* (`self.SpeedElevatorFloor`) -1.0)))))))

(fn `F_ElevatorFloor_Location`
  (params (`Delta Location X` :type "Float (double-precision)"))
  (`SceneComponent.K2_AddRelativeLocation` (`self.ElevatorFloor`) (`KismetMathLibrary.MakeVector` `Delta Location X`) false false))

(fn `UserConstructionScript`)