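; BP_Fan_2 is an interactive fan actor that spins while something overlaps its sphere collider.
; Begin and end overlap events on Sphere_FanCollision set and clear the OnRotate flag, without filtering which actor triggers them.
; While the flag is set, Tick calls FFanRotation, which adds Rotation times RotationSpeed to the Fan component's relative rotation.
; The step is not scaled by delta time, so spin speed depends on frame rate.
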(event `self.ReceiveTick`
  (params (DeltaSeconds :type "Float (single-precision)"))
  (if (`self.OnRotate`)
    (`self.F_FanRotation` (`self.Rotation`) (`self.RotationSpeed`))))

(event `self.Sphere_FanCollision.OnComponentBeginOverlap`
  (params (OverlappedComponent :type "PrimitiveComponent Object Reference") (OtherActor :type "Actor Object Reference") (OtherComp :type "PrimitiveComponent Object Reference") (OtherBodyIndex :type Integer) (bFromSweep :type Boolean) (SweepResult :type "HitResult Structure (by ref)"))
  ;[0 0 0] События коллайдера
  (set `self.OnRotate` true))

(event `self.Sphere_FanCollision.OnComponentEndOverlap`
  (params (OverlappedComponent :type "PrimitiveComponent Object Reference") (OtherActor :type "Actor Object Reference") (OtherComp :type "PrimitiveComponent Object Reference") (OtherBodyIndex :type Integer))
  ;[0 0 0] События коллайдера
  (set `self.OnRotate` false))

(fn `F_FanRotation`
  (params (RotationFan :type "Rotator Structure") (RotationSpeed :type "Float (double-precision)"))
  (`SceneComponent.K2_AddRelativeRotation` (`self.Fan`) (* RotationFan RotationSpeed) false false))

(fn `UserConstructionScript`)